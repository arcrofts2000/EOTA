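; BP_FixedCam is a fixed camera actor that becomes the player's view target when the character is inside its Box trigger.
; On BeginPlay, after a short delay, it takes the view if the first player's character already overlaps the box.
; Afterwards, any BP_ThirdPersonCharacter entering the box switches its own controller's view to this camera.
; Nothing restores the previous view when the character leaves.
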(event `self.ReceiveBeginPlay`
  (`KismetSystemLibrary.Delay` 0.2)
  (if (`PrimitiveComponent.IsOverlappingActor` (`self.Box`) (`GameplayStatics.GetPlayerCharacter` 0))
    (`PlayerController.SetViewTargetWithBlend` (`GameplayStatics.GetPlayerController` 0) self 0.0 "VTBlend_Linear" 0.0 false)))

(event `self.Box.OnComponentBeginOverlap`
  (params (OverlappedComponent :type "PrimitiveComponent Object Reference") (OtherActor :type "Actor Object Reference") (OtherComp :type "PrimitiveComponent Object Reference") (OtherBodyIndex :type Integer) (bFromSweep :type Boolean) (SweepResult :type "HitResult Structure (by ref)"))
  (bind _asbp_third_person_character (cast `/Game/ThirdPerson/Blueprints/BP_ThirdPersonCharacter` OtherActor))
  (`PlayerController.SetViewTargetWithBlend` (`PlayerState.GetPlayerController` (`Pawn.PlayerState` _asbp_third_person_character)) self 0.0 "VTBlend_Linear" 0.0 false))

(fn `UserConstructionScript`)